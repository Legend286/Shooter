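; Counter is an actor that destroys itself after taking a random number of hits.
; BeginPlay rolls a small random hit threshold, and each Hit event increments a running count against it.
; Debug strings print on every hit, including the final count just before the actor is destroyed.
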(event `self.ReceiveBeginPlay`
  (set `self.HitsRequired` (`KismetMathLibrary.RandomIntegerInRange` 1 8)))

(event `self.ReceiveHit`
  (params (MyComp :type "PrimitiveComponent Object Reference") (Other :type "Actor Object Reference") (OtherComp :type "PrimitiveComponent Object Reference") (bSelfMoved :type Boolean) (HitLocation :type "Vector Structure") (HitNormal :type "Vector Structure") (NormalImpulse :type "Vector Structure") (Hit :type "HitResult Structure (by ref)"))
  (bind _output_get (set `self.Hits` (+ (`self.Hits`) 1)))
  (if (>= (`self.Hits`) (`self.HitsRequired`))
    (`KismetSystemLibrary.PrintString` (`KismetTextLibrary.Conv_TextToString` (`|FormatText` "Destroying after {hits} hits" _output_get)))
    (`self.K2_DestroyActor`)
    (else
      (`KismetSystemLibrary.PrintString` "Hits += 1"))))

(fn `UserConstructionScript`)
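; Player controller for a sandbox mode that moves control from the starting editor pawn to a player pawn.
; It caches the initially controlled pawn on BeginPlay, and the F key calls SwitchPawn.
; SwitchPawn unpossesses, spawns a SandboxPlayerPawn above the world origin if none is valid, then possesses it.
; The switch is one-way, as the nodes that would repossess the editor pawn are disconnected.
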(event `self.ReceiveBeginPlay`
  (set `self.EditorPawn` (`self.K2_GetPawn`)))

(event `Key|F`
  (params (Key :type "Key Structure"))
  (:`Pressed`
    (`self.SwitchPawn`)))

(fn `SwitchPawn`
  (`self.UnPossess`)
  (if (not (`KismetSystemLibrary.IsValid` (`self.PlayerPawn`)))
    (bind _returnvalue (`|SpawnActorFromClass` "/Game/Blueprints/Game/SandboxPlayerPawn.SandboxPlayerPawn_C" (`KismetMathLibrary.MakeTransform` (0.0 0.0 500.0)) "Undefined" "OverrideRootScale" null null))
    (set `self.PlayerPawn` _returnvalue))
  (`self.Possess` (`self.PlayerPawn`)))

(fn `UserConstructionScript`)